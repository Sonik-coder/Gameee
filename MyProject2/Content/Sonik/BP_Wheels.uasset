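; BP_Wheels is an interactable wheel pickup that the player can attach to their character.
; On BeginPlay it looks up its RowName in the wheels data table and, if found, enables physics and applies that row's mesh.
; Interact snaps it to a socket on the player character's mesh, keeping world scale, then turns physics off and returns true.
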(event `self.ReceiveBeginPlay`
  (bind _staticmesh (`self.StaticMesh`))
  (bind _returnvalue (`|GetDataTableRow` "/Game/Sonik/WheelsDataTable.WheelsDataTable" (`self.Row Name`))
    (:`then`
      (`PrimitiveComponent.SetSimulatePhysics` _staticmesh true)
      (`StaticMeshComponent.SetStaticMesh` _staticmesh (`.Mesh_4_A02FEE254184BC756B3C92B31806957D` (break `/Game/Sonik/WheelsStruct` _returnvalue))))))

(fn `Interact`
  (returns (Interacted :type Boolean))
  (`self.K2_AttachToComponent` (`Character.Mesh` (`GameplayStatics.GetPlayerCharacter` 0)) "УEBU" "SnapToTarget" "SnapToTarget" "KeepWorld")
  (`PrimitiveComponent.SetSimulatePhysics` (`self.StaticMesh`) false)
  (return true))

(fn `UserConstructionScript`)